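; BP_Sight is a team-owned vision source that registers with the game's fog-of-war (FOW) manager.
; On BeginPlay it colors its sphere mesh to match its team, then registers itself as a sight provider through RiftGameState.
; Its sight-provider functions report the actor's location as origin, the SightRange variable as range, the team as tag, and mark it as non-static.
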(event `self.ReceiveBeginPlay`
  (switch `ERiftSightTag` (`self.MyTeam`)
    (:`None`
      (set `self.SphereMat` "/Game/SSH/Materials/Black.Black"))
    (:`Red`
      (set `self.SphereMat` "/Game/SSH/Materials/Red.Red"))
    (:`Blue`
      (set `self.SphereMat` "/Game/SSH/Materials/Blue.Blue")))
  (`PrimitiveComponent.SetMaterial` (`self.Sphere`) 0 (`self.SphereMat`))
  (bind _asrift_game_state (cast `RiftGameState` (`GameplayStatics.GetGameState`)))
  (`FOWManager.RegisterSightProvider` (`RiftGameState.GetFOWManager` _asrift_game_state) self))

(fn `GetSightOrigin`
  (returns (ReturnValue :type "Vector Structure"))
  (return (`self.K2_GetActorLocation`)))

(fn `GetSightRange`
  (returns (ReturnValue :type "Float (single-precision)"))
  (return (`self.SightRange`)))

(fn `GetSightTag`
  (returns (ReturnValue :type "ERiftSightTag Enum"))
  (return (`self.MyTeam`)))

(fn `IsStatic`
  (returns (ReturnValue :type Boolean))
  (return false))

(fn `UserConstructionScript`)